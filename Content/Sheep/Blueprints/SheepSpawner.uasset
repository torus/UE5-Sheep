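; SheepSpawner is an actor that fills the level with sheep, spawning them one at a time at its own transform.
; BeginPlay starts a Spawn event that creates a Sheep, waits half a second, increments Count and prints it.
; The event then calls itself until Count reaches 300, using the Delay to pace the loop.
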(event `self.ReceiveBeginPlay`
  (`self.spawn`))

(event `spawn`
  (`|SpawnActorFromClass` "/Game/Sheep/Blueprints/Sheep.Sheep_C" (`self.GetTransform`) "Undefined" "MultiplyWithRoot" null null)
  (`KismetSystemLibrary.Delay` 0.5)
  (bind _result (`/Engine/EditorBlueprintResources/StandardMacros.IncrementInt` (`self.count`))
    (:`  `
      (`KismetSystemLibrary.PrintText` (`|FormatText` "count: {c}" _result) true false (struct :`G` 0.66 :`B` 1.0 :`A` 1.0) 0.5)
      (if (< (`self.count`) 300)
        (`self.spawn`)))))

(fn `UserConstructionScript`)